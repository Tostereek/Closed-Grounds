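; Game mode for Closed Grounds that drives a fog value over the course of a day and handles player death.
; While counting from BeginPlay, Tick lerps fog from a start value toward a threshold over the day duration, broadcasting updates until complete.
; Day manager's day-ended event stops and resets the countdown; quest manager's all-finished event plays a sound.
; Player death triggers the character's restart; GAS kill logic is left disconnected.
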(event `self.ReceiveTick`
  (params (DeltaSeconds :type "Float (single-precision)"))
  (`self.IsCounting`
    (:`then`
      (set `self.ElapsedTime` (+ (`self.ElapsedTime`) (`GameplayStatics.GetWorldDeltaSeconds`)))
      (set `self.Alpha` (`KismetMathLibrary.FClamp` (`KismetMathLibrary.SafeDivide` (`self.ElapsedTime`) (`self.DayDuration`))))
      (set `self.CurrentFogValue` (`KismetMathLibrary.Lerp` (`self.StartFogValue`) (`self.FogTreshold`) (`self.Alpha`)))
      (if (>= (`self.Alpha`) 1.0)
        (set `self.IsCounting` false)
        (else
          (`self.OnFogUpdate` (`self.CurrentFogValue`)))))
    (:`else`)))

(event `OnDayEnded_Event`
  (`self.ResetFog`))

(event `self.ReceiveBeginPlay`
  (`parent.ReceiveBeginPlay`)
  (add `CG_QuestManager.OnFinishedAllQuests` (subsystem `CG_QuestManager`) (delegate `OnFinishedAllQuests_Event`))
  (`self.StartCountdown`)
  (add `CG_DayManager.OnDayEnded` (subsystem `CG_DayManager`) (delegate `OnDayEnded_Event`)))

(event `OnFinishedAllQuests_Event`
  (`GameplayStatics.PlaySound2D` "/Game/PlaceholderAssets/A_CWLmuwi.A_CWLmuwi" 1.0 1.0 0.0 null null))

(event `self.HandlePlayerDeath`
  (`parent.HandlePlayerDeath`)
  (bind _asbp_player_character (cast `/Game/ClosedGrounds/Blueprints/Characters/Player/BP_PlayerCharacter` (`GameplayStatics.GetPlayerCharacter` 0)))
  (`/Game/ClosedGrounds/Blueprints/Characters/Player/BP_PlayerCharacter.OnRestartGame` _asbp_player_character))

(fn `ResetFog`
  (set `self.IsCounting` false)
  (set `self.CurrentFogValue` (`self.StartFogValue`))
  (set `self.ElapsedTime` 0.0)
  (return))

(fn `StartCountdown`
  (set `self.IsCounting` true)
  (return))

(fn `UserConstructionScript`)