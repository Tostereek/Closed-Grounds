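; Gameplay Ability for a dash that launches the avatar along its forward vector with a short constant root motion force and a dash sound.
; On activation it commits, caches the camera and default FOV, and adds a dynamic speedlines material as a post-process blendable.
; When the force finishes it starts a short end-ability timer, and ending the ability removes the blendable.
; The FOV kick is present but disconnected.
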(event `self.K2_ActivateAbility`
  (bind _returnvalue (`self.K2_CommitAbility`))
  (if _returnvalue
    (`self.CacheCamera`)
    (`self.CacheDefaultFOV`)
    (`self.ShowVignette`)
    (`GameplayStatics.PlaySound2D` "/Game/PlaceholderAssets/Art/Sounds/Characters/Chain/Dash/A_Dash.A_Dash" 1.0 1.0 0.0 null null)
    (`AbilityTask_ApplyRootMotionConstantForce.ApplyRootMotionConstantForce` "None" (`Actor.GetActorForwardVector` (`self.GetAvatarActorFromActorInfo`)) 2750.0 0.3 false null "MaintainLastRootMotionVelocity" (0.0 0.0 0.0) 500.0
      (:`OnFinish`
        (`self.OnFinishDash`)))
    (else
      (`KismetSystemLibrary.PrintString` "Ability wasn't commited!")
      (`self.K2_EndAbility`))))

(event `OnFinishDash`
  (bind _returnvalue (`KismetSystemLibrary.K2_SetTimerDelegate` (`|CreateDelegate` :!event `K2_EndAbility`) 0.3))
  (set `self.EndAbility_TimerHandle` _returnvalue))

(event `self.K2_OnEndAbility`
  (params (bWasCancelled :type Boolean))
  (`CameraComponent.RemoveBlendable` (`self.Camera`) (`self.DashVFX`)))

(fn `CacheCamera`
  (set `self.Camera` (`Actor.GetComponentByClass` (`self.GetAvatarActorFromActorInfo`) "/Script/Engine.CameraComponent"))
  (return))

(fn `CacheDefaultFOV`
  (set `self.DefualtFOV` (`CameraComponent.FieldOfView` (`self.Camera`))))

(fn `ChangeFOV`
  (params (InNewFOV :type "Float (double-precision)"))
  (`CameraComponent.SetFieldOfView` (`self.Camera`) (+ (`self.DefualtFOV`) (`local.InNewFOV`)))
  (return))

(fn `ShowVignette`
  (bind _returnvalue (`KismetMaterialLibrary.CreateDynamicMaterialInstance` "/Game/ClosedGrounds/Art/MaterialLibrary/M_Dash_Speedlines.M_Dash_Speedlines"))
  (bind _output_get (set `self.DashVFX` _returnvalue))
  (`CameraComponent.AddOrUpdateBlendable` (`self.Camera`) _output_get 1.0))