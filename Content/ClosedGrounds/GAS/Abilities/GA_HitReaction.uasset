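; Gameplay Ability that plays a character's hit reaction: a hurt montage, a sound and a brief material flash.
; On commit it caches the avatar and its slot 0 mesh material, then swaps in the flash material.
; A BlinkTime timer restores the material and ends the ability, which also ends when the montage finishes or is interrupted.
; Ending clears the timer without restoring the material itself.
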(event `self.K2_ActivateAbility`
  (`parent.K2_ActivateAbility`)
  (bind _returnvalue (`self.K2_CommitAbility`))
  (if _returnvalue
    (`self.CacheAvatarActor`)
    (`self.CacheAvatarMeshMaterial`)
    (`self.PlayHitReactionSound`)
    (`self.ChangeToFlashMaterial`)
    (bind _returnvalue_2 (`KismetSystemLibrary.K2_SetTimerDelegate` (`|CreateDelegate` :!event `OnBackToDefaultMaterial`) (`self.BlinkTime`)))
    (set `self.ChangeToDefaultMaterial_TimerHandle` _returnvalue_2)
    (`AbilityTask_PlayMontageAndWait.CreatePlayMontageAndWaitProxy` "None" "/Game/ClosedGrounds/Art/Characters/Chain/A_Chain_1H_Hurt_Montage.A_Chain_1H_Hurt_Montage"
      (:`OnCompleted`
        _)
      (:`OnInterrupted`
        _)
      (:`OnCancelled`
        _))
    (`self.K2_EndAbility`)
    (else
      (`self.K2_EndAbility`))))

(event `OnBackToDefaultMaterial`
  (`self.ChangeToDefaultMaterial`)
  (`self.K2_EndAbility`))

(event `self.K2_OnEndAbility`
  (params (bWasCancelled :type Boolean))
  (`KismetSystemLibrary.K2_ClearAndInvalidateTimerHandle` (`self.ChangeToDefaultMaterial_TimerHandle`)))

(fn `CacheAvatarActor`
  (bind _ascg_character_base (cast `CG_CharacterBase` (`self.GetAvatarActorFromActorInfo`)))
  (set `self.AvatarActor` _ascg_character_base)
  (return))

(fn `CacheAvatarMeshMaterial`
  (set `self.MeshMaterial` (`PrimitiveComponent.GetMaterial` (`Character.Mesh` (`self.AvatarActor`)) 0))
  (return))

(fn `ChangeToDefaultMaterial`
  (`PrimitiveComponent.SetMaterial` (`Character.Mesh` (`self.AvatarActor`)) 0 (`self.MeshMaterial`))
  (return))

(fn `ChangeToFlashMaterial`
  (`PrimitiveComponent.SetMaterial` (`Character.Mesh` (`self.AvatarActor`)) 0 (`self.FlashMateial`))
  (return))

(fn `PlayHitReactionSound`
  (`GameplayStatics.PlaySoundAtLocation` (`self.SFX_HitReaction`) (`Actor.K2_GetActorLocation` (`self.AvatarActor`)) (struct) 1.0 1.0 0.0 null null null null)
  (return))